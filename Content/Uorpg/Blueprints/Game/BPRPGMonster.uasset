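; BPRPGMonster is an RPG monster Blueprint that moves to a position handed to it.
; MoveToPosition, apparently an interface function, stores the target, sets a Move flag and triggers the MovePosition event.
; That event casts the instigator controller to BPRPG_AIController, issues an AI move to the target and prints debug messages on failure or finish.
; Alternative move calls are left unconnected, and Tick is empty.
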(event Custom|Move%20Position
  (bind _asbprpg_aicontroller (Utilities|Casting|CastToBPRPG_AIController (Game|GetInstigatorController)))
  (AI|AIMoveTo _asbprpg_aicontroller (Variables|Default|GetTargetPosition) 0 -1.0 "Default" "Default" true true
    (:OnRequestFailed
      (Development|PrintString "failed move"))
    (:OnMoveFinished
      (Development|PrintString "Finish move"))))

(event EventBeginPlay)

(event EventActorBeginOverlap
  (params (OtherActor :type Actor%20Object%20Reference)))

(event EventTick
  (params (DeltaSeconds :type Float%20%28single-precision%29)))

(fn ConstructionScript
  (|CallParentFunction))

(fn MovetoPosition
  (params (In%20Position :type Vector))
  (bind _output_get (Variables|Default|SetTargetPosition In%20Position))
  (Variables|Default|SetbMove true)
  (Development|PrintString "Move Inferface")
  (CallFunction|MovePosition)
  (return _output_get))