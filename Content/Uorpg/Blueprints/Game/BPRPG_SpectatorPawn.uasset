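; RTS-style spectator pawn that box-selects units and orders them to move.
; Clicks are located by tracing along the camera's forward vector rather than from the cursor, with debug lines drawn.
; Left-drag endpoints form an XY box that gathers all Pawns inside into Units, with Left Shift appending.
; A right-click whose press and release hits match sends each unit a MoveToPosition interface message; direct AI move nodes are left unwired.
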(event Custom|Check%20Select%20Units
  (bind _firstposition (Variables|Default|GetFirstPosition))
  (bind _lastposition (Variables|Default|GetLastPosition))
  (bind (_x _y _z) (Math|Vector|BreakVector _lastposition))
  (bind (_x_2 _y_2 _z_2) (Math|Vector|BreakVector _firstposition))
  (if (not (Math|Vector|Equal(Vector) _firstposition _lastposition 0.0001))
    ;[1 1 1] Min & Max Select Vector
    (bind _output_get (Variables|Default|SetMinPosition (Math|Vector|MakeVector (Math|Float|Min(Float) _x_2 _x) (Math|Float|Min(Float) _y_2 _y) (Math|Float|Min(Float) _z_2 _z))))
    (bind _output_get_2 (Variables|Default|SetMaxPosition (Math|Vector|MakeVector (Math|Float|Max(Float) _x_2 _x) (Math|Float|Max(Float) _y_2 _y) (Math|Float|Max(Float) _z_2 _z))))
    (Development|PrintString (Utilities|String|Append "Min:" (Utilities|String|ToString(Vector) _output_get)) true true "(R=0.000000,G=0.660000,B=1.000000,A=1.000000)" 2.0)
    (Development|PrintString (Utilities|String|Append "Max:" (Utilities|String|ToString(Vector) _output_get_2)) true true "(R=0.000000,G=0.660000,B=1.000000,A=1.000000)" 2.0)
    (if (Variables|Default|GetbSelected)
      _
      (else
        (Utilities|Array|Clear (Variables|Default|GetUnits))))
    (bind _outactors (Actor|GetAllActorsOfClass "/Script/Engine.Pawn"))
    (for _array_element _outactors
      (if (Math|Boolean|ANDBoolean (Math|Float|InRange(Float) (.X (Math|Vector|BreakVector (Transformation|GetActorLocation _array_element))) (.X (Math|Vector|BreakVector (Variables|Default|GetMinPosition))) (.X (Math|Vector|BreakVector (Variables|Default|GetMaxPosition)))) (Math|Float|InRange(Float) (.Y (Math|Vector|BreakVector (Transformation|GetActorLocation _array_element))) (.Y (Math|Vector|BreakVector (Variables|Default|GetMinPosition))) (.Y (Math|Vector|BreakVector (Variables|Default|GetMaxPosition)))) true)
        (Development|PrintString (Utilities|String|Append "Found: " (Utilities|GetDisplayName _array_element)))
        (Utilities|Array|Add (Variables|Default|GetUnits) _array_element)))))

(event Custom|Move%20Units
  ;[1 1 1] Check Mouse Right Position to move
  (if (Math|Vector|Equal(Vector) (Variables|Default|GetMouseRightPosition01) (Variables|Default|GetMouseRightPosition02) 0.0001)
    (Development|PrintString "Move units?")
    (for _array_element (Variables|Default|GetUnits)
      (Class|BPMoveCommand|MovetoPosition(Message) _array_element (Variables|Default|GetMouseRightPosition02)))))

(event EventBeginPlay)

(event EventActorBeginOverlap
  (params (OtherActor :type Actor%20Object%20Reference)))

(event EventTick
  (params (DeltaSeconds :type Float%20%28single-precision%29))
  (bind _returnvalue (Game|GetPlayerCameraManager 0))
  (bind _returnvalue_2 (Camera|GetCameraLocation _returnvalue))
  (Collision|LineTraceByChannel _returnvalue_2 (+ _returnvalue_2 (* (Math|Vector|GetForwardVector (Camera|GetCameraRotation _returnvalue)) 1.5e+03)) "TraceTypeQuery1" false 0 "ForOneFrame"))

(event Input|MouseEvents|LeftMouseButton
  (params (Key :type Key%20Structure :default "AnyKey"))
  (bind _returnvalue (Game|GetPlayerCameraManager 0))
  (bind _returnvalue_2 (Camera|GetCameraRotation _returnvalue))
  (bind _returnvalue_3 (Camera|GetCameraLocation _returnvalue))
  (bind _returnvalue_4 (Math|Vector|GetForwardVector _returnvalue_2))
  (bind _returnvalue_5 (* _returnvalue_4 1.5e+03))
  (bind _returnvalue_6 (+ _returnvalue_3 _returnvalue_5))
  ;[1 1 1] Select Mouse Units
  (:Pressed
    (Development|PrintString "mouse down")
    (bind (_outhit _returnvalue_7) (Collision|LineTraceByChannel _returnvalue_3 _returnvalue_6 "TraceTypeQuery1" false 0 "ForOneFrame"))
    (if _returnvalue_7
      (Development|PrintString (Utilities|String|Append "Pos:" (Utilities|String|ToString(Vector) (.Location (Collision|BreakHitResult _outhit)))) false false)
      (Variables|Default|SetFirstPosition (.Location (Collision|BreakHitResult _outhit)))))
  (:Released
    (bind (_outhit_2 _returnvalue_8) (Collision|LineTraceByChannel _returnvalue_3 _returnvalue_6 "TraceTypeQuery1" false 0 "ForOneFrame"))
    (if _returnvalue_8
      (Development|PrintString (Utilities|String|Append "Pos:" (Utilities|String|ToString(Vector) (.Location (Collision|BreakHitResult _outhit_2)))) false false)
      (Variables|Default|SetLastPosition (.Location (Collision|BreakHitResult _outhit_2)))
      (CallFunction|CheckSelectUnits))))

(event Input|KeyboardEvents|LeftShift
  (params (Key :type Key%20Structure :default "AnyKey"))
  ;[1 1 1] Key press for adding units
  (:Pressed
    (Variables|Default|SetbSelected true))
  (:Released
    (Variables|Default|SetbSelected false)))

(event Input|MouseEvents|RightMouseButton
  (params (Key :type Key%20Structure :default "AnyKey"))
  (bind _returnvalue (Game|GetPlayerCameraManager 0))
  (bind _returnvalue_2 (Camera|GetCameraRotation _returnvalue))
  (bind _returnvalue_3 (Camera|GetCameraLocation _returnvalue))
  (bind _returnvalue_4 (Math|Vector|GetForwardVector _returnvalue_2))
  (bind _returnvalue_5 (* _returnvalue_4 1.5e+03))
  (bind _returnvalue_6 (+ _returnvalue_3 _returnvalue_5))
  ;[1 1 1] Mouse Right Press/Release Position
  (:Pressed
    (bind (_outhit _returnvalue_7) (Collision|LineTraceByChannel _returnvalue_3 _returnvalue_6 "TraceTypeQuery1" false 0 "ForOneFrame"))
    (if _returnvalue_7
      (Development|PrintString (Utilities|String|Append "Pos:" (Utilities|String|ToString(Vector) (.Location (Collision|BreakHitResult _outhit)))) false false)
      (Variables|Default|SetMouseRightPosition01 (.Location (Collision|BreakHitResult _outhit)))))
  (:Released
    (bind (_outhit_2 _returnvalue_8) (Collision|LineTraceByChannel _returnvalue_3 _returnvalue_6 "TraceTypeQuery1" false 0 "ForOneFrame"))
    (if _returnvalue_8
      (Development|PrintString (Utilities|String|Append "Pos:" (Utilities|String|ToString(Vector) (.Location (Collision|BreakHitResult _outhit_2)))) false false)
      (Variables|Default|SetMouseRightPosition02 (.Location (Collision|BreakHitResult _outhit_2)))
      (CallFunction|MoveUnits))))

(fn ConstructionScript)