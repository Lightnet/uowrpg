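; BPRPG_SaveGame is the RPG save game object that stores the player's name, status, stats, inventories and the open level name.
; SavePlayerState copies the name, status, stats and inventories from a given PlayerState into its own variables.
; Getters and setters expose the player name and open level name, while the inventory getter and setter are empty stubs.
; The open level name is set separately through its setter.
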(fn GetPlayerInventories
  (return 0))

(fn SetPlayerInventories
  (params (In%20Inventories :type Array%20of%20Actor%20Object%20References)))

(fn GetOpenLevel
  (return (Variables|Default|GetOpen%20Level%20Name)))

(fn SetOpenLevel
  (params (In%20Name :type String))
  (Variables|Default|SetOpen%20Level%20Name In%20Name))

(fn GetPlayerName
  (return (Variables|Default|GetPlayerName)))

(fn SetPlayerName
  (params (In%20Name :type String))
  (Variables|Default|SetPlayerName In%20Name))

(fn SavePlayerState
  (params (Player%20State :type BPRPG%20Player%20State%20Object%20Reference))
  (Variables|Default|SetPlayerName (Variables|/Game/Uorpg/Blueprints/Game/BPRPG_PlayerState.BPRPG_PlayerState_C|GetPlayer Player%20State))
  (Variables|Default|SetPlayer%20Status (Variables|/Game/Uorpg/Blueprints/Game/BPRPG_PlayerState.BPRPG_PlayerState_C|GetPlayerStatus Player%20State))
  (Variables|Default|SetPlayer%20Stats (Variables|/Game/Uorpg/Blueprints/Game/BPRPG_PlayerState.BPRPG_PlayerState_C|GetPlayerStats Player%20State))
  (Variables|Default|SetPlayer%20Inventories (Variables|/Game/Uorpg/Blueprints/Game/BPRPG_PlayerState.BPRPG_PlayerState_C|GetInventories Player%20State)))