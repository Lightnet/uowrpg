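; RPG player state that holds the player's name, status and quest list.
; On BeginPlay it spawns a BPRPG_Quest_Simple actor at the world origin into Quests, then copies name and status from the SaveGame held by BPRPG_GameInstance.
; Loading prints the saved name on screen, and a separate DisplayPlayerID debug event, not called here, prints PlayerName.
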(event Custom|Display%20Player%20ID
  ;[1 1 1] Player ID print
  (Development|PrintString (Utilities|String|Append "Init playerstate:" (Variables|Default|GetPlayerName))))

(event Custom|Load%20Player%20State%20FIle
  ;[1 1 1] Load player game file
  (bind _asbprpg_game_instance (Utilities|Casting|CastToBPRPG_GameInstance (Game|GetGameInstance)))
  (Development|PrintString (Utilities|String|Append "Player:" (Variables|/Game/Uorpg/Blueprints/Game/BPRPG_SaveGame.BPRPG_SaveGame_C|GetPlayerName (Variables|/Game/Uorpg/Blueprints/Game/BPRPG_GameInstance.BPRPG_GameInstance_C|GetSaveGame _asbprpg_game_instance))) true true "(R=0.685000,G=0.368481,B=0.000000,A=1.000000)" 5.0)
  (Variables|Default|SetPlayer (Variables|/Game/Uorpg/Blueprints/Game/BPRPG_SaveGame.BPRPG_SaveGame_C|GetPlayerName (Variables|/Game/Uorpg/Blueprints/Game/BPRPG_GameInstance.BPRPG_GameInstance_C|GetSaveGame _asbprpg_game_instance)))
  (Variables|Default|Setplayerstatus (Variables|/Game/Uorpg/Blueprints/Game/BPRPG_SaveGame.BPRPG_SaveGame_C|Getplayerstatus (Variables|/Game/Uorpg/Blueprints/Game/BPRPG_GameInstance.BPRPG_GameInstance_C|GetSaveGame _asbprpg_game_instance))))

(event Custom|Init%20Quest
  ;[1 1 1] Init Quest
  (bind _returnvalue (Game|SpawnActorfromClass "/Game/Uorpg/Blueprints/Object/quests/BPRPG_Quest_Simple.BPRPG_Quest_Simple_C" (Math|Transform|MakeTransform "0, 0, 0") "Undefined" 0 0))
  (Utilities|Array|Add (Variables|Default|Getquests) _returnvalue))

(event EventBeginPlay
  ;[1 1 1] Being Play
  (CallFunction|InitQuest)
  (CallFunction|LoadPlayerStateFIle))

(event EventTick
  (params (DeltaSeconds :type Float%20%28single-precision%29)))

(fn ConstructionScript)