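; Online RPG game mode that handles player names when play begins and when players join.
; On BeginPlay, after a short delay, it sends the game instance's PlayerName to player controller 0 through an interface message and prints it for debugging.
; On PostLogin, after the same delay, it tells the joining RPG player controller to check its name.
; Disconnected debug chains for server/client status and player-name listing remain in the graph but never run.
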(event EventPostLogin
  (params (NewPlayer :type Player%20Controller%20Object%20Reference))
  (Utilities|FlowControl|Delay 0.2)
  (bind _asbprpg_player_controller (Utilities|Casting|CastToBPRPG_PlayerController NewPlayer))
  (Default|CheckPlayerName _asbprpg_player_controller))

(event EventBeginPlay
  (Utilities|FlowControl|Delay 0.2)
  (bind _asbprpg_game_instance (Utilities|Casting|CastToBPRPG_GameInstance (Game|GetGameInstance)))
  (Class|BPIPlayerName|IChangePlayerName(Message) (Game|GetPlayerController 0) (Variables|/Game/Uorpg/Blueprints/Game/BPRPG_GameInstance.BPRPG_GameInstance_C|GetPlayerName _asbprpg_game_instance))
  (Development|PrintString (Utilities|String|Append "GAME INSTNACE?:" (Variables|/Game/Uorpg/Blueprints/Game/BPRPG_GameInstance.BPRPG_GameInstance_C|GetPlayerName _asbprpg_game_instance)) true true "(R=0.000000,G=0.660000,B=1.000000,A=1.000000)" 1e+01))

(fn ConstructionScript)