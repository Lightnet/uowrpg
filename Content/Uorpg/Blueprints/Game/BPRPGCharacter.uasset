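; RPG character Blueprint that shows a floating name and HP readout and takes damage.
; Every Tick it refreshes both texts from the Status struct and yaws them to face the player camera.
; AnyDamage prints debug text with the instigator's name and subtracts damage from HealthPoint, with no clamping or death handling.
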(event EventBeginPlay)

(event EventActorBeginOverlap
  (params (OtherActor :type Actor%20Object%20Reference)))

(event EventTick
  (params (DeltaSeconds :type Float%20%28single-precision%29))
  (bind _returnvalue (Game|GetPlayerCameraManager 0))
  (bind _returnvalue_2 (Transformation|GetActorLocation))
  (bind _displayhealth (Variables|Default|GetDisplayHealth))
  (bind _displayname (Variables|Default|GetDisplayName))
  (bind _status (Variables|Default|GetStatus))
  (bind (_name _healthpoint _maxhealthpoint) (Utilities|Struct|BreakSStatus _status))
  (bind _returnvalue_3 (Camera|GetCameraLocation _returnvalue))
  (bind _returnvalue_4 (Math|Rotator|FindLookatRotation _returnvalue_2 _returnvalue_3))
  (bind _yaw (Math|Rotator|BreakRotator _returnvalue_4))
  (Rendering|Components|TextRender|SetText _displayname (Utilities|Text|ToText(String) _name))
  (Rendering|Components|TextRender|SetText _displayhealth (Utilities|Text|ToText(String) (Utilities|String|Append "HP:" (Utilities|String|ToString(Float) _healthpoint) "/" (Utilities|String|ToString(Float) _maxhealthpoint))))
  (Transformation|SetWorldRotation _displayname (Math|Rotator|MakeRotator 0.0 0.0 _yaw) false false)
  (Transformation|SetWorldRotation _displayhealth (Math|Rotator|MakeRotator 0.0 0.0 _yaw) false false))

(event Game|Damage|EventAnyDamage
  (params (Damage :type Float%20%28single-precision%29) (DamageType :type Damage%20Type%20Object%20Reference) (InstigatedBy :type Controller%20Object%20Reference) (DamageCauser :type Actor%20Object%20Reference))
  (bind _status (Variables|Default|GetStatus))
  (Development|PrintString (Utilities|GetDisplayName InstigatedBy))
  (Development|PrintString "Any Damage")
  (Utilities|Struct|SetmembersinSStatus _status (- (.HealthPoint (Utilities|Struct|BreakSStatus _status)) Damage)))

(event Game|Damage|EventPointDamage
  (params (Damage :type Float%20%28single-precision%29) (DamageType :type Damage%20Type%20Object%20Reference) (HitLocation :type Vector :default "0, 0, 0") (HitNormal :type Vector :default "0, 0, 0") (HitComponent :type Primitive%20Component%20Object%20Reference) (BoneName :type Name :default "None") (ShotFromDirection :type Vector :default "0, 0, 0") (InstigatedBy :type Controller%20Object%20Reference) (DamageCauser :type Actor%20Object%20Reference)))

(event Game|Damage|EventRadialDamage
  (params (DamageReceived :type Float%20%28single-precision%29) (DamageType :type Damage%20Type%20Object%20Reference) (Origin :type Vector :default "0, 0, 0") (HitInfo :type Hit%20Result%20Structure%20%28by%20ref%29) (InstigatedBy :type Controller%20Object%20Reference) (DamageCauser :type Actor%20Object%20Reference)))

(fn ConstructionScript)