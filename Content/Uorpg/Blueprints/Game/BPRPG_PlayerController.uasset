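; RPG player controller that relays the player's name to and from BPRPG_PlayerState.
; Interface-style IChangePlayerName and IGetPlayerName cast the PlayerState and write or return its Player value.
; SetPlayerName stores and prints a separate local PlayerName without updating the PlayerState, and CheckPlayerName prints the PlayerState name in red for debugging.
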(event Custom|SetPlayerName
  (params (PlayerName :type String))
  (bind _output_get (Variables|Default|SetPlayerName PlayerName))
  (Development|PrintString _output_get))

(event Custom|Check%20Player%20Name
  (bind _asbprpg_player_state (Utilities|Casting|CastToBPRPG_PlayerState (Variables|GetPlayerState)))
  (Development|PrintString (Variables|/Game/Uorpg/Blueprints/Game/BPRPG_PlayerState.BPRPG_PlayerState_C|GetPlayer _asbprpg_player_state) true true "(R=1.000000,G=0.106508,B=0.000000,A=1.000000)"))

(event EventBeginPlay)

(event EventTick
  (params (DeltaSeconds :type Float%20%28single-precision%29)))

(event EventIChangePlayerName
  (params (Name :type String))
  (bind _asbprpg_player_state (Utilities|Casting|CastToBPRPG_PlayerState (Variables|GetPlayerState)))
  (Variables|/Game/Uorpg/Blueprints/Game/BPRPG_PlayerState.BPRPG_PlayerState_C|SetPlayer _asbprpg_player_state Name))

(fn ConstructionScript)

(fn IGetPlayerName
  (bind _asbprpg_player_state (Utilities|Casting|CastToBPRPG_PlayerState (Variables|GetPlayerState)))
  (return (Variables|/Game/Uorpg/Blueprints/Game/BPRPG_PlayerState.BPRPG_PlayerState_C|GetPlayer _asbprpg_player_state)))