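; RPG game instance that manages named player save profiles and audio volume settings.
; Profiles live in indexed, prefixed slots; each operation scans a fixed slot range matching PlayerName to create (first free slot), list, load, save or delete.
; Loading stores the SaveGame, shows a loading screen and opens TestingArea; saving writes a fresh save object via SavePlayerState.
; Init applies a base sound mix after a delay, and volume events override its per-category sound classes.
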(event Custom|UI%20Change
  (params (Audio%20Volume :type Float%20%28single-precision%29))
  ;[1 1 1] Audio Chnage Event
  (bind _output_get (Variables|Default|SetUI%20Volume Audio%20Volume))
  (Audio|SetSoundMixClassOverride "/Game/Uorpg/Audios/BPSoundMix.BPSoundMix" "/Game/Uorpg/Audios/UI_VolumeClass.UI_VolumeClass" _output_get 1.0 1.0 true))

(event Custom|Voice%20Change
  (params (Audio%20Volume :type Float%20%28single-precision%29))
  ;[1 1 1] Audio Chnage Event
  (bind _output_get (Variables|Default|SetVoice%20Volume Audio%20Volume))
  (Audio|SetSoundMixClassOverride "/Game/Uorpg/Audios/BPSoundMix.BPSoundMix" "/Game/Uorpg/Audios/Voice_VolumeClass.Voice_VolumeClass" _output_get 1.0 1.0 true))

(event Custom|Init%20Master%20Sound
  ;[1 1 1] Init Sound
  (Utilities|FlowControl|Delay 1.0)
  (Class|GameplayStatics|SetBaseSoundMix "/Game/Uorpg/Audios/BPSoundMix.BPSoundMix"))

(event Custom|Save%20Player%20Name%20Game
  (params (PlayerName :type String))
  ;[1 1 1] Save Player Name Game Data
  (for _index (range 0 10)
    (bind _returnvalue (SaveGame|DoesSaveGameExist (Utilities|String|Append (Variables|Default|GetPrefix_Player) (Utilities|String|ToString(Integer) _index))))
    (if _returnvalue
      (bind _returnvalue_2 (SaveGame|LoadGamefromSlot (Utilities|String|Append (Variables|Default|GetPrefix_Player) (Utilities|String|ToString(Integer) _index))))
      (bind _asbprpg_save_game (Utilities|Casting|CastToBPRPG_SaveGame _returnvalue_2))
      (if (Utilities|Enum|Equal(Enum) PlayerName (Variables|/Game/Uorpg/Blueprints/SaveGame/BPRPG_SaveGame.BPRPG_SaveGame_C|GetPlayerName _asbprpg_save_game))
        (bind _returnvalue_3 (SaveGame|CreateSaveGameObject "/Game/Uorpg/Blueprints/SaveGame/BPRPG_SaveGame.BPRPG_SaveGame_C"))
        (Variables|/Game/Uorpg/Blueprints/SaveGame/BPRPG_SaveGame.BPRPG_SaveGame_C|SetPlayerName _returnvalue_3 PlayerName)
        (Utilities|Casting|CastToBPRPG_PlayerState (Variables|/Script/Engine.Controller|GetPlayerState (Game|GetPlayerController 0)))
        (Default|SavePlayerState _returnvalue_3)
        (SaveGame|SaveGametoSlot _returnvalue_3 (Utilities|String|Append (Variables|Default|GetPrefix_Player) (Utilities|String|ToString(Integer) _index)))
        (Development|PrintString (Utilities|String|Append "Save Game!" (Utilities|String|Append (Variables|Default|GetPrefix_Player) (Utilities|String|ToString(Integer) _index))) false false "(R=1.000000,G=0.039766,B=0.000000,A=1.000000)" 5.0)))))

(event Custom|Change%20Volume
  (params (Audio%20Volume :type Float%20%28single-precision%29))
  ;[1 1 1] Audio Chnage Event
  (bind _output_get (Variables|Default|SetAudio%20Volume Audio%20Volume))
  (Audio|SetSoundMixClassOverride "/Game/Uorpg/Audios/BPSoundMix.BPSoundMix" "/Game/Uorpg/Audios/Master_VolumeClass.Master_VolumeClass" _output_get 1.0 1.0 true))

(event Custom|Music%20Change
  (params (Audio%20Volume :type Float%20%28single-precision%29))
  ;[1 1 1] Audio Chnage Event
  (bind _output_get (Variables|Default|SetMusic%20Volume Audio%20Volume))
  (Audio|SetSoundMixClassOverride "/Game/Uorpg/Audios/BPSoundMix.BPSoundMix" "/Game/Uorpg/Audios/Music_VolumeClass.Music_VolumeClass" _output_get 1.0 1.0 true))

(event Custom|Sound%20Effect%20Change
  (params (Audio%20Volume :type Float%20%28single-precision%29))
  ;[1 1 1] Audio Chnage Event
  (bind _output_get (Variables|Default|SetSound%20Effects%20Volume Audio%20Volume))
  (Audio|SetSoundMixClassOverride "/Game/Uorpg/Audios/BPSoundMix.BPSoundMix" "/Game/Uorpg/Audios/FX_VolumeClass.FX_VolumeClass" _output_get 1.0 1.0 true))

(event Custom|Delete%20Player%20Name
  (params (Index :type Integer) (playername :type String))
  ;[1 1 1] Delete Player Name
  (for _index (range 0 10)
    (bind _returnvalue (SaveGame|DoesSaveGameExist (Utilities|String|Append (Variables|Default|GetPrefix_Player) (Utilities|String|ToString(Integer) _index))))
    (if _returnvalue
      (bind _returnvalue_2 (SaveGame|LoadGamefromSlot (Utilities|String|Append (Variables|Default|GetPrefix_Player) (Utilities|String|ToString(Integer) _index))))
      (bind _asbprpg_save_game (Utilities|Casting|CastToBPRPG_SaveGame _returnvalue_2))
      (if (Utilities|Enum|Equal(Enum) playername (Variables|/Game/Uorpg/Blueprints/SaveGame/BPRPG_SaveGame.BPRPG_SaveGame_C|GetPlayerName _asbprpg_save_game))
        (bind _returnvalue_3 (SaveGame|DeleteGameinSlot (Utilities|String|Append (Variables|Default|GetPrefix_Player) (Utilities|String|ToString(Integer) _index))))
        (if _returnvalue_3
          (Development|PrintString "Delete Player")
          (else
            (Development|PrintString "Error ?")))))))

(event Custom|Save%20Player%20Name
  (params (Name :type String))
  ;[1 1 1] Save Game Player Name
  (Utilities|Array|Clear (Variables|Default|GetSaveSlots))
  (Variables|Default|SetbFoundPlayer false)
  (for _index (range 0 10)
    (bind _returnvalue (SaveGame|DoesSaveGameExist (Utilities|String|Append (Variables|Default|GetPrefix_Player) (Utilities|String|ToString(Integer) _index))))
    (if _returnvalue
      (Utilities|Array|Add (Variables|Default|GetSaveSlots) (Utilities|String|Append (Variables|Default|GetPrefix_Player) (Utilities|String|ToString(Integer) _index)))
      (bind _returnvalue_2 (SaveGame|LoadGamefromSlot (Utilities|String|Append (Variables|Default|GetPrefix_Player) (Utilities|String|ToString(Integer) _index))))
      (bind _asbprpg_save_game (Utilities|Casting|CastToBPRPG_SaveGame _returnvalue_2))
      (if (Utilities|Enum|Equal(Enum) Name (Variables|/Game/Uorpg/Blueprints/SaveGame/BPRPG_SaveGame.BPRPG_SaveGame_C|GetPlayerName _asbprpg_save_game))
        (Variables|Default|SetbFoundPlayer true)
        (Development|PrintString "Player File Exist!" false false))))
  (if (not (Variables|Default|GetbFoundPlayer))
    (bind _index_2 (Utilities|FlowControl|ForLoopwithBreak 0 10 :!label _label)
      (:LoopBody
        (Variables|Default|SetIsSlot false)
        (bind _array_element (Utilities|Array|ForEachLoopwithBreak (Variables|Default|GetSaveSlots) :!label _label_2)
          (:LoopBody
            (if (Utilities|Enum|Equal(Enum) (Utilities|String|Append (Variables|Default|GetPrefix_Player) (Utilities|String|ToString(Integer) _index_2)) _array_element)
              (Variables|Default|SetIsSlot true)
              (goto _label_2 Break)))
          (:Completed
            (if (not (Variables|Default|GetIsSlot))
              (bind _returnvalue_3 (SaveGame|CreateSaveGameObject "/Game/Uorpg/Blueprints/SaveGame/BPRPG_SaveGame.BPRPG_SaveGame_C"))
              (Variables|/Game/Uorpg/Blueprints/SaveGame/BPRPG_SaveGame.BPRPG_SaveGame_C|SetPlayerName _returnvalue_3 Name)
              (SaveGame|SaveGametoSlot _returnvalue_3 (Utilities|String|Append (Variables|Default|GetPrefix_Player) (Utilities|String|ToString(Integer) _index_2)))
              (goto _label Break))))))))

(event Custom|Load%20Player%20Name
  (params (PlayerName :type String))
  ;[1 1 1] Load Player Name
  (for _index (range 0 10)
    (bind _returnvalue (SaveGame|DoesSaveGameExist (Utilities|String|Append (Variables|Default|GetPrefix_Player) (Utilities|String|ToString(Integer) _index))))
    (if _returnvalue
      (bind _returnvalue_2 (SaveGame|LoadGamefromSlot (Utilities|String|Append (Variables|Default|GetPrefix_Player) (Utilities|String|ToString(Integer) _index))))
      (bind _asbprpg_save_game (Utilities|Casting|CastToBPRPG_SaveGame _returnvalue_2))
      (if (Utilities|Enum|Equal(Enum) PlayerName (Variables|/Game/Uorpg/Blueprints/SaveGame/BPRPG_SaveGame.BPRPG_SaveGame_C|GetPlayerName _asbprpg_save_game))
        (Variables|Default|SetSaveGame _asbprpg_save_game)
        (bind _returnvalue_3 (UserInterface|CreateWidget "/Game/Uorpg/Blueprints/Widgets/BPWLoadingScreen.BPWLoadingScreen_C"))
        (UserInterface|Viewport|AddtoViewport _returnvalue_3 0)
        (Input|SetInputModeGameOnly (Game|GetPlayerController 0))
        (Utilities|FlowControl|Delay 0.2)
        (Game|OpenLevel(byName) "TestingArea")))))

(event EventInit
  ;[1 1 1] Init
  (CallFunction|InitMasterSound)
  (Development|PrintString "RPG Game Instance" false false))

(fn ListPlayerNames
  (Utilities|Array|Clear (LocalVariables|GetPlayerNames))
  (for _index (range 0 10)
    (bind _returnvalue (SaveGame|DoesSaveGameExist (Utilities|String|Append (Variables|Default|GetPrefix_Player) (Utilities|String|ToString(Integer) _index))))
    (if _returnvalue
      (bind _returnvalue_2 (SaveGame|LoadGamefromSlot (Utilities|String|Append (Variables|Default|GetPrefix_Player) (Utilities|String|ToString(Integer) _index))))
      (bind _asbprpg_save_game (Utilities|Casting|CastToBPRPG_SaveGame _returnvalue_2))
      (Utilities|Array|Add (LocalVariables|GetPlayerNames) (Variables|/Game/Uorpg/Blueprints/SaveGame/BPRPG_SaveGame.BPRPG_SaveGame_C|GetPlayerName _asbprpg_save_game))))
  (return (LocalVariables|GetPlayerNames)))