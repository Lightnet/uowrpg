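; RPG HUD Blueprint that puts the player HUD and hotbar on screen and manages the game's menu widgets.
; Toggle events for inventory, storage, NPC, bank, build, skills and interact prompts lazily create and cache widgets, then add or remove them.
; Most menus also switch cursor, click events and input mode.
; Other events handle dungeon menu and HUD, HUD removal, and job-class selection, which shares the DungeonHUD variable.
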(event Custom|Add%20Dungeon%20HUD
  ;[1 1 1] Dungeon Hud
  (Utilities|IsValid (Variables|Default|GetDungeonHUD)
    (:Is%20Valid
      _)
    (:Is%20Not%20Valid
      (bind _returnvalue (UserInterface|CreateWidget "/Game/Uorpg/Blueprints/Widgets/BPWDungeonHUD.BPWDungeonHUD_C"))
      (Variables|Default|SetDungeonHUD _returnvalue)))
  (UserInterface|Viewport|AddtoViewport (Variables|Default|GetDungeonHUD) 0))

(event Custom|Toggle%20Skills%20Menu
  (params (bShow :type Boolean) (Actor :type Actor%20Object%20Reference))
  (bind _returnvalue (Game|GetPlayerController 0))
  (bind _returnvalue_2 (Game|GetPlayerController 0))
  ;[1 1 1] Skill Menu
  (if bShow
    (Utilities|IsValid (Variables|Default|GetWidget_Skills)
      (:Is%20Valid
        _)
      (:Is%20Not%20Valid
        (bind _returnvalue_3 (UserInterface|CreateWidget "/Game/Uorpg/Blueprints/Widgets/BPWShopPanel01.BPWShopPanel01_C"))
        (Variables|Default|SetWidget_Skills _returnvalue_3)))
    (Utilities|IsValid (Variables|Default|GetWidget_Skills)
      (:Is%20Valid
        (UserInterface|Viewport|AddtoViewport (Variables|Default|GetWidget_Skills) 0)
        (Variables|/Script/Engine.PlayerController|SetbEnableClickEvents _returnvalue_2 true)
        (Variables|/Script/Engine.PlayerController|SetbShowMouseCursor _returnvalue_2 true)))
    (else
      (Utilities|IsValid (Variables|Default|GetWidget_Skills)
        (:Is%20Valid
          (Widget|RemovefromParent (Variables|Default|GetWidget_Skills))
          (Variables|/Script/Engine.PlayerController|SetbEnableClickEvents _returnvalue false)
          (Variables|/Script/Engine.PlayerController|SetbShowMouseCursor _returnvalue false)
          (Input|SetInputModeGameOnly _returnvalue))))))

(event Custom|ToggleWidgetStorage
  (params (bShow :type Boolean) (Actor :type Actor%20Object%20Reference))
  (bind _returnvalue (Game|GetPlayerController 0))
  (bind _returnvalue_2 (Game|GetPlayerController 0))
  ;[1 1 1] Widget Storage
  (if bShow
    (Utilities|IsValid (Variables|Default|GetWidgetStorage)
      (:Is%20Valid
        _)
      (:Is%20Not%20Valid
        (bind _returnvalue_3 (UserInterface|CreateWidget "/Game/Uorpg/Blueprints/Widgets/BPWidgetStorage.BPWidgetStorage_C"))
        (Variables|Default|SetWidgetStorage _returnvalue_3)))
    (Utilities|IsValid (Variables|Default|GetWidgetStorage)
      (:Is%20Valid
        (Class|BPRPGActor|SetObject(Message) (Variables|Default|GetWidgetStorage) Actor)
        (UserInterface|Viewport|AddtoViewport (Variables|Default|GetWidgetStorage) 0)
        (Variables|/Script/Engine.PlayerController|SetbEnableClickEvents _returnvalue true)
        (Variables|/Script/Engine.PlayerController|SetbShowMouseCursor _returnvalue true)
        (Input|SetInputModeGameandUI _returnvalue (Variables|Default|GetWidgetStorage) "DoNotLock" false)))
    (else
      (Utilities|IsValid (Variables|Default|GetWidgetStorage)
        (:Is%20Valid
          (Widget|RemovefromParent (Variables|Default|GetWidgetStorage))
          (Variables|/Script/Engine.PlayerController|SetbEnableClickEvents _returnvalue_2 false)
          (Variables|/Script/Engine.PlayerController|SetbShowMouseCursor _returnvalue_2 false)
          (Input|SetInputModeGameOnly _returnvalue_2))))))

(event Custom|JobClassEvent
  (bind _returnvalue (Game|GetPlayerController 0))
  ;[1 1 1] Job Class Hud
  (Utilities|IsValid (Variables|Default|GetDungeonHUD)
    (:Is%20Valid
      _)
    (:Is%20Not%20Valid
      (bind _returnvalue_2 (UserInterface|CreateWidget "/Game/Uorpg/Blueprints/Widgets/BPWSelectJobClassMenu.BPWSelectJobClassMenu_C"))
      (bind _output_get (Variables|Default|SetDungeonHUD _returnvalue_2))))
  (UserInterface|Viewport|AddtoViewport (Variables|Default|GetDungeonHUD) 0)
  (Variables|/Script/Engine.PlayerController|SetbShowMouseCursor _returnvalue true)
  (Variables|/Script/Engine.PlayerController|SetbEnableClickEvents _returnvalue true)
  (Input|SetInputModeGameandUI _returnvalue _output_get "DoNotLock" true))

(event Custom|ToggleWidgetNPC
  (params (bShow :type Boolean) (Actor :type Actor%20Object%20Reference))
  (bind _returnvalue (Game|GetPlayerController 0))
  (bind _returnvalue_2 (Game|GetPlayerController 0))
  ;[1 1 1] ToggleWidgetNPC
  (if bShow
    (Utilities|IsValid (Variables|Default|GetWidgetNPC)
      (:Is%20Valid
        _)
      (:Is%20Not%20Valid
        (bind _returnvalue_3 (UserInterface|CreateWidget "/Game/Uorpg/Blueprints/Widgets/BPNPCMenu.BPNPCMenu_C"))
        (Variables|Default|SetWidgetNPC _returnvalue_3)))
    (Utilities|IsValid (Variables|Default|GetWidgetNPC)
      (:Is%20Valid
        (UserInterface|Viewport|AddtoViewport (Variables|Default|GetWidgetNPC) 0)
        (Variables|/Script/Engine.PlayerController|SetbEnableClickEvents _returnvalue true)
        (Variables|/Script/Engine.PlayerController|SetbShowMouseCursor _returnvalue true)
        (Input|SetInputModeGameandUI _returnvalue (Variables|Default|GetWidgetNPC) "DoNotLock" false)))
    (else
      (Utilities|IsValid (Variables|Default|GetWidgetNPC)
        (:Is%20Valid
          (Widget|RemovefromParent (Variables|Default|GetWidgetNPC))
          (Variables|/Script/Engine.PlayerController|SetbEnableClickEvents _returnvalue_2 false)
          (Variables|/Script/Engine.PlayerController|SetbShowMouseCursor _returnvalue_2 false)
          (Input|SetInputModeGameOnly _returnvalue_2))))))

(event Custom|Remove%20HUDs
  ;[1 1 1] Remove HUDs
  (Widget|RemovefromParent (Variables|Default|GetHUDPlayer))
  (Widget|RemovefromParent (Variables|Default|GetWidgetHotKeys))
  (Widget|RemovefromParent (Variables|Default|GetDungeonHUD)))

(event Custom|ToggleWidgetBank
  (params (bShow :type Boolean) (Actor :type Actor%20Object%20Reference))
  (bind _returnvalue (Game|GetPlayerController 0))
  (bind _returnvalue_2 (Game|GetPlayerController 0))
  ;[1 1 1] ToggleWidgetBank
  (if bShow
    (Utilities|IsValid (Variables|Default|GetWidgetBank)
      (:Is%20Valid
        _)
      (:Is%20Not%20Valid
        (bind _returnvalue_3 (UserInterface|CreateWidget "/Game/Uorpg/Blueprints/Widgets/BPWidgetBank.BPWidgetBank_C"))
        (Variables|Default|SetWidgetBank _returnvalue_3)))
    (Utilities|IsValid (Variables|Default|GetWidgetBank)
      (:Is%20Valid
        (UserInterface|Viewport|AddtoViewport (Variables|Default|GetWidgetBank) 0)
        (Variables|/Script/Engine.PlayerController|SetbEnableClickEvents _returnvalue true)
        (Variables|/Script/Engine.PlayerController|SetbShowMouseCursor _returnvalue true)
        (Input|SetInputModeGameandUI _returnvalue (Variables|Default|GetWidgetBank) "DoNotLock" false)))
    (else
      (Utilities|IsValid (Variables|Default|GetWidgetBank)
        (:Is%20Valid
          (Widget|RemovefromParent (Variables|Default|GetWidgetBank))
          (Variables|/Script/Engine.PlayerController|SetbEnableClickEvents _returnvalue_2 false)
          (Variables|/Script/Engine.PlayerController|SetbShowMouseCursor _returnvalue_2 false)
          (Input|SetInputModeGameOnly _returnvalue_2))))))

(event Custom|DungeonMenuWidget
  (bind _returnvalue (Game|GetPlayerController 0))
  ;[1 1 1] Dugneon Menu
  (Utilities|IsValid (Variables|Default|GetDungeonMenu)
    (:Is%20Valid
      _)
    (:Is%20Not%20Valid
      (bind _returnvalue_2 (UserInterface|CreateWidget "/Game/Uorpg/Blueprints/Widgets/BPDungeonMenu.BPDungeonMenu_C"))
      (Variables|Default|SetDungeonMenu _returnvalue_2)))
  (UserInterface|Viewport|AddtoViewport (Variables|Default|GetDungeonMenu) 0)
  (Variables|/Script/Engine.PlayerController|SetbShowMouseCursor _returnvalue true)
  (Variables|/Script/Engine.PlayerController|SetbEnableClickEvents _returnvalue true)
  (Input|SetInputModeUIOnly _returnvalue (Variables|Default|GetDungeonMenu) "DoNotLock"))

(event Custom|Add%20Player%20HUD
  ;[1 1 1] Add Player HUD
  (UserInterface|Viewport|AddtoViewport (Variables|Default|GetHUDPlayer) 0)
  (UserInterface|Viewport|AddtoViewport (Variables|Default|GetWidgetHotKeys) 0))

(event Custom|ToggleWidgetBuildMode
  (params (bShow :type Boolean) (Actor :type Actor%20Object%20Reference))
  (bind _returnvalue (Game|GetPlayerController 0))
  (bind _returnvalue_2 (Game|GetPlayerController 0))
  ;[1 1 1] ToggleWidgetBuildMode
  (if bShow
    (Utilities|IsValid (Variables|Default|GetWidgetBuildMode)
      (:Is%20Valid
        _)
      (:Is%20Not%20Valid
        (bind _returnvalue_3 (UserInterface|CreateWidget "/Game/Uorpg/Blueprints/Widgets/BPWidgetBuildMenu.BPWidgetBuildMenu_C"))
        (Variables|Default|SetWidgetBuildMode _returnvalue_3)))
    (Utilities|IsValid (Variables|Default|GetWidgetBuildMode)
      (:Is%20Valid
        (UserInterface|Viewport|AddtoViewport (Variables|Default|GetWidgetBuildMode) 0)
        (Variables|/Script/Engine.PlayerController|SetbEnableClickEvents _returnvalue true)
        (Variables|/Script/Engine.PlayerController|SetbShowMouseCursor _returnvalue true)
        (Input|SetInputModeGameandUI _returnvalue (Variables|Default|GetWidgetBuildMode) "DoNotLock" true)))
    (else
      (Utilities|IsValid (Variables|Default|GetWidgetBuildMode)
        (:Is%20Valid
          (Widget|RemovefromParent (Variables|Default|GetWidgetBuildMode))
          (Variables|/Script/Engine.PlayerController|SetbEnableClickEvents _returnvalue_2 false)
          (Variables|/Script/Engine.PlayerController|SetbShowMouseCursor _returnvalue_2 false)
          (Input|SetInputModeGameOnly _returnvalue_2))))))

(event Custom|Toggle%20Inventory%20Menu
  (params (bShow :type Boolean))
  (bind _returnvalue (Game|GetPlayerController 0))
  (bind _returnvalue_2 (Game|GetPlayerController 0))
  ;[1 1 1] Inventory Toggle
  (if bShow
    (Utilities|IsValid (Variables|Default|GetWidgetInventory)
      (:Is%20Valid
        _)
      (:Is%20Not%20Valid
        (bind _returnvalue_3 (UserInterface|CreateWidget "/Game/Uorpg/Blueprints/Widgets/BPWGameMenuAccess.BPWGameMenuAccess_C"))
        (Variables|Default|SetWidgetInventory _returnvalue_3)))
    (Utilities|IsValid (Variables|Default|GetWidgetInventory)
      (:Is%20Valid
        (UserInterface|Viewport|AddtoViewport (Variables|Default|GetWidgetInventory) 0)
        (Variables|/Script/Engine.PlayerController|SetbEnableClickEvents _returnvalue true)
        (Variables|/Script/Engine.PlayerController|SetbShowMouseCursor _returnvalue true)
        (Input|SetInputModeGameandUI _returnvalue (Variables|Default|GetWidgetInventory) "DoNotLock" true)))
    (else
      (Utilities|IsValid (Variables|Default|GetWidgetInventory)
        (:Is%20Valid
          (Widget|RemovefromParent (Variables|Default|GetWidgetInventory))
          (Variables|/Script/Engine.PlayerController|SetbEnableClickEvents _returnvalue_2 false)
          (Variables|/Script/Engine.PlayerController|SetbShowMouseCursor _returnvalue_2 false)
          (Input|SetInputModeGameOnly _returnvalue_2))))))

(event Custom|HoverWidgetInteract
  (params (bShow :type Boolean) (Actor :type Actor%20Object%20Reference))
  (bind _returnvalue (Game|GetPlayerController 0))
  ;[1 1 1] ToggleWidget Interact
  (if bShow
    (Utilities|IsValid (Variables|Default|GetWidget_Interact)
      (:Is%20Valid
        _)
      (:Is%20Not%20Valid
        (bind _returnvalue_2 (UserInterface|CreateWidget "/Game/Uorpg/Blueprints/Widgets/BPWidgetInteract.BPWidgetInteract_C" 0 Actor))
        (Variables|Default|SetWidget_Interact _returnvalue_2)))
    (Utilities|IsValid (Variables|Default|GetWidget_Interact)
      (:Is%20Valid
        (bind _asbpwidget_interact (Utilities|Casting|CastToBPWidgetInteract (Variables|Default|GetWidget_Interact)))
        (Variables|/Game/Uorpg/Blueprints/Widgets/BPWidgetInteract.BPWidgetInteract_C|SetActor _asbpwidget_interact Actor)
        (if (not (Widget|IsVisible (Variables|Default|GetWidget_Interact)))
          (UserInterface|Viewport|AddtoViewport (Variables|Default|GetWidget_Interact) 0))))
    (else
      (Utilities|IsValid (Variables|Default|GetWidget_Interact)
        (:Is%20Valid
          (Widget|RemovefromParent (Variables|Default|GetWidget_Interact))
          (Variables|/Script/Engine.PlayerController|SetbEnableClickEvents _returnvalue false)
          (Variables|/Script/Engine.PlayerController|SetbShowMouseCursor _returnvalue false)
          (Input|SetInputModeGameOnly _returnvalue))))))

(event EventBeginPlay
  ;[1 1 1] Begin play
  (bind _returnvalue (UserInterface|CreateWidget "/Game/Uorpg/Blueprints/Widgets/PlayerHUD.PlayerHUD_C"))
  (UserInterface|Viewport|AddtoViewport _returnvalue 0)
  (Variables|Default|SetHUDPlayer _returnvalue)
  (bind _returnvalue_2 (UserInterface|CreateWidget "/Game/Uorpg/Blueprints/Widgets/BPW_HotBarAccess.BPW_HotBarAccess_C"))
  (UserInterface|Viewport|AddtoViewport _returnvalue_2 0)
  (Variables|Default|SetWidgetHotKeys _returnvalue_2))

(event EventActorBeginOverlap
  (params (OtherActor :type Actor%20Object%20Reference)))

(event EventTick
  (params (DeltaSeconds :type Float%20%28single-precision%29)))

(fn ConstructionScript)