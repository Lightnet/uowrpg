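; RPG game mode that restores the player's saved state from the game instance's save game when a start spot is initialized.
; InitStartSpot acts only for player controller 0, passing the save to the PlayerState through SetPlayerStateMessage.
; If that succeeds and LoadTransformSaveGame is set, it waits briefly, then applies the saved transform to the pawn and the saved rotation to the controller.
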(event EventBeginPlay)

(event EventTick
  (params (DeltaSeconds :type Float%20%28single-precision%29)))

(event EventHandleStartingNewPlayer
  (params (NewPlayer :type Player%20Controller%20Object%20Reference))
  ;[1 1 1] Nothing here...
)

(event EventInitStartSpot
  (params (StartSpot :type Actor%20Object%20Reference) (NewPlayer :type Controller%20Object%20Reference))
  (bind _returnvalue (Game|GetPlayerController 0))
  ;[1 1 1] Load Player state from save game data
  (bind _asbprpg_game_instance (Utilities|Casting|CastToBPRPG_GameInstance (Game|GetGameInstance)))
  (Development|PrintString (Utilities|String|Append "Player Name:" (Variables|/Script/Engine.PlayerState|GetPlayerName (Variables|/Script/Engine.Controller|GetPlayerState NewPlayer))) false false "(R=1.000000,G=0.000000,B=0.212421,A=1.000000)")
  (Development|PrintString (Utilities|String|Append "Player Name:" (Variables|/Script/Engine.PlayerState|GetPlayerName (Variables|/Script/Engine.Controller|GetPlayerState _returnvalue))) false false "(R=0.964126,G=0.000000,B=1.000000,A=1.000000)")
  (if (== NewPlayer _returnvalue)
    (Development|PrintString "Pass Controller" false false)
    ;;[1 1 1] Player Start Actor
    (Development|PrintString (Utilities|GetDisplayName StartSpot) false false "(R=1.000000,G=0.084660,B=0.000000,A=1.000000)")
    (if (Utilities|IsValid _asbprpg_game_instance)
      (bind _ispass (Class|BPIRPGPlayerState|SetPlayerState(Message) :self (Variables|/Script/Engine.Controller|GetPlayerState NewPlayer) :Save%20Game (Variables|/Game/Uorpg/Blueprints/Game/BPRPG_GameInstance.BPRPG_GameInstance_C|GetSaveGame _asbprpg_game_instance)))
      (if _ispass
        (Development|PrintString "Pass Save" false false "(R=0.000000,G=1.000000,B=0.250000,A=1.000000)")
        (Development|PrintString (Utilities|String|Append "GM Player Name" "") false false "(R=0.810000,G=0.000000,B=0.007096,A=1.000000)")
        (if (Variables|/Game/Uorpg/Blueprints/Game/BPRPG_GameInstance.BPRPG_GameInstance_C|GetbLoadTransformSaveGame _asbprpg_game_instance)
          (Utilities|FlowControl|Delay 1.0)
          ;;[1 1 1] Set Pawn Location
          (Transformation|SetActorTransform (Pawn|GetControlledPawn NewPlayer) (Math|Transform|MakeTransform (.Location (Math|Transform|BreakTransform (Variables|/Game/Uorpg/Blueprints/SaveGame/BPRPG_SaveGame.BPRPG_SaveGame_C|GetPlayer%20Transform (Variables|/Game/Uorpg/Blueprints/Game/BPRPG_GameInstance.BPRPG_GameInstance_C|GetSaveGame _asbprpg_game_instance)))) (.Rotation (Math|Transform|BreakTransform (Variables|/Game/Uorpg/Blueprints/SaveGame/BPRPG_SaveGame.BPRPG_SaveGame_C|GetPlayer%20Transform (Variables|/Game/Uorpg/Blueprints/Game/BPRPG_GameInstance.BPRPG_GameInstance_C|GetSaveGame _asbprpg_game_instance)))) (.Scale (Math|Transform|BreakTransform (Variables|/Game/Uorpg/Blueprints/SaveGame/BPRPG_SaveGame.BPRPG_SaveGame_C|GetPlayer%20Transform (Variables|/Game/Uorpg/Blueprints/Game/BPRPG_GameInstance.BPRPG_GameInstance_C|GetSaveGame _asbprpg_game_instance))))))
          (Development|PrintString (Utilities|String|Append "HERE? Position:" (Utilities|String|ToString(Vector) (.Location (Math|Transform|BreakTransform (Variables|/Game/Uorpg/Blueprints/SaveGame/BPRPG_SaveGame.BPRPG_SaveGame_C|GetPlayer%20Transform (Variables|/Game/Uorpg/Blueprints/Game/BPRPG_GameInstance.BPRPG_GameInstance_C|GetSaveGame _asbprpg_game_instance)))))) false false "(R=1.000000,G=0.048188,B=0.000000,A=1.000000)" 5.0)
          (Development|PrintString (Utilities|String|Append "ROT:" (Utilities|String|ToString(Rotator) (.Rotation (Math|Transform|BreakTransform (Variables|/Game/Uorpg/Blueprints/SaveGame/BPRPG_SaveGame.BPRPG_SaveGame_C|GetPlayer%20Transform (Variables|/Game/Uorpg/Blueprints/Game/BPRPG_GameInstance.BPRPG_GameInstance_C|GetSaveGame _asbprpg_game_instance)))))) false false "(R=1.000000,G=0.048188,B=0.000000,A=1.000000)" 5.0)
          ;;[1 1 1] Controller Set Rotate
          (Pawn|SetControlRotation NewPlayer (.Rotation (Math|Transform|BreakTransform (Variables|/Game/Uorpg/Blueprints/SaveGame/BPRPG_SaveGame.BPRPG_SaveGame_C|GetPlayer%20Transform (Variables|/Game/Uorpg/Blueprints/Game/BPRPG_GameInstance.BPRPG_GameInstance_C|GetSaveGame _asbprpg_game_instance))))))
        (else
          (Development|PrintString "Fail Save" false false))))
    (else
      (Development|PrintString "Fail Controller" false false))))

(fn ConstructionScript)