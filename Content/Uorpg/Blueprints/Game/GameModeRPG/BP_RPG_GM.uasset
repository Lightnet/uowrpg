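; RPG game mode Blueprint that keeps a list of player controllers.
; OnSwapPlayerControllers adds each new controller to AllPlayerControllers, while InitStartSpot and RespawnPlayer are empty stubs.
; An unconnected chain, which never runs, holds save loading: it applies the game instance's save to the PlayerState, then optionally restores pawn transform and, after a short delay, control rotation.
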(event Custom|RespawnPlayer
  (params (PlayerController :type Player%20Controller%20Object%20Reference) (PlayerCharacter :type Character%20Class%20Reference)))

(event EventInitStartSpot
  (params (StartSpot :type Actor%20Object%20Reference) (NewPlayer :type Controller%20Object%20Reference))
  ;[1 1 1] Load Player state from save game data
)

(event EventOnSwapPlayerControllers
  (params (OldPC :type Player%20Controller%20Object%20Reference) (NewPC :type Player%20Controller%20Object%20Reference))
  ;[1 1 1] Keep Track of connect Player Controller
  (Utilities|Array|Add (Variables|GameInfo|GetAllPlayerControllers) NewPC))

(fn ConstructionScript)