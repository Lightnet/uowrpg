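; DataTable01 is an actor that spawns the item prefabs listed in the DTRPG_Item data table when play begins.
; BeginPlay loops over every row name, looks up the row and, where its PrefabItem class is valid, spawns that class at this actor's location with default rotation and scale.
; All items land at the same point; a leftover item-name print is disconnected.
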(event EventBeginPlay
  (bind _outrownames (DataTable|GetDataTableRowNames "/Game/Uorpg/Blueprints/Game/Database/DTRPG_Item.DTRPG_Item"))
  (for _array_element _outrownames
    (bind _returnvalue (Utilities|GetDataTableRow "/Game/Uorpg/Blueprints/Game/Database/DTRPG_Item.DTRPG_Item" _array_element)
      (:then
        (if (Utilities|IsValidClass (Utilities|ResolveSoftReference (.PrefabItem (Utilities|Struct|BreakRPGItem _returnvalue))))
          (Game|SpawnActorfromClass (Utilities|ResolveSoftReference (.PrefabItem (Utilities|Struct|BreakRPGItem _returnvalue))) (Math|Transform|MakeTransform (Transformation|GetActorLocation)) "Undefined" 0 0))))))

(event Collision|EventActorBeginOverlap
  (params (OtherActor :type Actor%20Object%20Reference)))

(event EventTick
  (params (DeltaSeconds :type Float%20%28single-precision%29)))

(fn ConstructionScript)