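; Fireball projectile Blueprint that damages RPG objects it overlaps.
; CharacterActor stores the owning actor in CharActor so the Box overlap can ignore the shooter.
; Overlapping another BPRPG_Object applies a small fixed damage and destroys the projectile, while other actors leave it alive.
; The Box hit event only prints, and debug prints trace owner assignment and overlaps.
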(event OnComponentBeginOverlap(Box)
  (params (OverlappedComponent :type Primitive%20Component%20Object%20Reference) (OtherActor :type Actor%20Object%20Reference) (OtherComp :type Primitive%20Component%20Object%20Reference) (OtherBodyIndex :type Integer) (bFromSweep :type Boolean) (SweepResult :type Hit%20Result%20Structure%20%28by%20ref%29))
  (Development|PrintString "Hit O")
  (Development|PrintString (Utilities|String|Append "Character Owner set?:" (Utilities|GetDisplayName (Variables|Default|GetCharActor))))
  (Development|PrintString (Utilities|String|Append "hit set?:" (Utilities|GetDisplayName OtherActor)))
  (if (!= (Variables|Default|GetCharActor) OtherActor)
    (Utilities|Casting|CastToBPRPG_Object OtherActor)
    (Game|Damage|ApplyDamage OtherActor 1.0 0 0)
    (Development|PrintString "desotry bullet")
    (Actor|DestroyActor)))

(event OnComponentHit(Box)
  (params (HitComponent :type Primitive%20Component%20Object%20Reference) (OtherActor :type Actor%20Object%20Reference) (OtherComp :type Primitive%20Component%20Object%20Reference) (NormalImpulse :type Vector :default "0, 0, 0") (Hit :type Hit%20Result%20Structure%20%28by%20ref%29))
  (Development|PrintString "Hit"))

(event EventBeginPlay)

(event Collision|EventActorBeginOverlap
  (params (OtherActor :type Actor%20Object%20Reference)))

(event EventTick
  (params (DeltaSeconds :type Float%20%28single-precision%29)))

(fn ConstructionScript)

(fn CharacterActor
  (params (SetActor :type Actor%20Object%20Reference))
  (Development|PrintString (Utilities|String|Append "owener pawn projectile" (Utilities|GetDisplayName SetActor)) true false)
  (bind _output_get (Variables|Default|SetCharActor SetActor))
  (return _output_get))