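; BPRPG_Object is an RPG world object that holds item data and exposes it for interaction and pickup.
; Setters and getters handle base info, held item, owner, icon, messages, hand-item data and the pickup flag.
; Hovering forwards the actor to BPRPG_HUD to show or hide its interact widget.
; SetObject and GetObjectItem are empty stubs, and GetBaseInfo returns zero buy cost instead of the stored BuyPrice.
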(event EventHoverInterface
  (params (Actor :type Actor%20Object%20Reference) (bShow :type Boolean))
  ;[1 1 1] Interact Object
  (bind _asbprpg_hud (Utilities|Casting|CastToBPRPG_HUD (HUD|GetHUD (Game|GetPlayerController 0))))
  (Default|HoverWidgetInteract _asbprpg_hud bShow Actor))

(event EventISetItem
  (params (InItem :type Actor%20Object%20Reference))
  (Variables|Default|SetItem%20Holder InItem))

(event EventSetBaseInfo
  (params (ItemID :type String) (Name :type String) (Description :type String) (bstack :type Boolean) (Types :type Array%20of%20Strings) (BuyCost :type Float%20%28single-precision%29) (SellCost :type Float%20%28single-precision%29) (Stack :type Integer) (MaxStack :type Integer))
  (Variables|Default|SetItemID ItemID)
  (Variables|Default|SetName Name)
  (Variables|Default|SetDescription Description)
  (Variables|Default|SetbStack bstack)
  (Variables|Default|SetBuyPrice BuyCost)
  (Variables|Default|SetSellPrice SellCost)
  (Variables|Default|SetStack Stack)
  (Variables|Default|SetMaxStack MaxStack))

(event EventBeginPlay)

(event EventActorBeginOverlap
  (params (OtherActor :type Actor%20Object%20Reference)))

(event EventTick
  (params (DeltaSeconds :type Float%20%28single-precision%29)))

(fn ConstructionScript)

(fn SetObject
  (return))

(fn GetObjectItem
  (return))

(fn CharacterActor
  (params (SetActor :type Actor%20Object%20Reference))
  (bind _output_get (Variables|Default|SetOwnerActor SetActor))
  (return _output_get))

(fn GetBaseInfo
  (return (Variables|Default|GetItemID) (Variables|Default|GetName) (Variables|Default|GetDescription) (Variables|Default|GetbStack) (Variables|Default|GetKeywords) 0.0 (Variables|Default|GetSellPrice) (Variables|Default|GetStack) (Variables|Default|GetMaxStack) (Variables|Default|GetTypes)))

(fn GetIcon
  (return (Variables|Default|GetIconTexture2D)))

(fn GetMessages
  (return (Variables|Default|GetInteractMessages)))

(fn IGetDataItem
  (return (Variables|Default|GetClass%20Item) (Variables|Default|GetIs%20Dominant%20Hand) (Variables|Default|GetAnimationHandName)))

(fn IGetItem
  (return (Variables|Default|GetItem%20Holder)))

(fn PickupObject
  (return (Variables|Default|GetEnablePickup)))