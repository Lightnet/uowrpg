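; BPRPG_Object_Cube is an interactable storage object that holds an inventory of item actors.
; On BeginPlay it spawns an actor for each class in ClassItems at the world origin and adds it to its Items array.
; InteractObject gets BPRPG_HUD from the first player controller and opens the storage widget with itself as the source, then prints a debug message.
; GetInventories and SetInventories read and replace the Items array.
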(event EventBeginPlay
  (for _array_element (Variables|Default|GetClass%20Items)
    (bind _returnvalue (Game|SpawnActorfromClass _array_element (Math|Transform|MakeTransform "0, 0, 0") "Undefined" 0 0))
    (Utilities|Array|Add (Variables|Default|GetItems) _returnvalue)))

(event EventActorBeginOverlap
  (params (OtherActor :type Actor%20Object%20Reference)))

(event EventTick
  (params (DeltaSeconds :type Float%20%28single-precision%29)))

(event EventInteractObject
  (params (Actor :type Actor%20Object%20Reference))
  (bind _asbprpg_hud (Utilities|Casting|CastToBPRPG_HUD (HUD|GetHUD (Game|GetPlayerController 0))))
  (Default|ToggleWidgetStorage _asbprpg_hud true self)
  (Development|PrintString "Hit Cube "))

(fn ConstructionScript
  (|CallParentFunction))

(fn GetInventories
  (return (Variables|Default|GetItems)))

(fn SetInventories
  (params (Items%20In :type Array%20of%20Actor%20Object%20References))
  (bind _output_get (Variables|Default|SetItems Items%20In))
  (return _output_get))