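; BPRPG_SaveGame is the RPG's save object, storing player name, level name to open and inventory records.
; SavePlayerState copies the name and flattens each inventory item's base info into SRPGInventory structs, typing equip or weapon items separately and printing each entry.
; LoadInventory matches saved IDs against the DTRPG_IDItems table but does nothing on a match.
; Accessors expose saved fields, though Get/SetPlayerInventories are empty stubs.
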(event Custom|Save%20PlayerState
  (params (playerstate :type BPRPG%20Player%20State%20Object%20Reference))
  (Variables|Default|SetPlayerName (Variables|/Game/Uorpg/Blueprints/Game/BPRPG_PlayerState.BPRPG_PlayerState_C|GetPlayer playerstate))
  (CallFunction|SaveInventories (Variables|/Game/Uorpg/Blueprints/Game/BPRPG_PlayerState.BPRPG_PlayerState_C|GetInventories playerstate)))

(event Custom|Load%20Inventory
  ;[1 1 1] Can't Spawn here
  (for _array_element (Variables|Default|GetSPlayer%20Inventories)
    (bind _outrownames (DataTable|GetDataTableRowNames "/Game/Uorpg/Blueprints/SaveGame/DTRPG_IDItems.DTRPG_IDItems"))
    (bind _array_element_2 (Utilities|Array|ForEachLoopwithBreak _outrownames)
      (:LoopBody
        (bind _returnvalue (Utilities|GetDataTableRow "/Game/Uorpg/Blueprints/SaveGame/DTRPG_IDItems.DTRPG_IDItems" _array_element_2)
          (:then
            (if (Utilities|Enum|Equal(Enum) (.ItemID (Utilities|Struct|BreakSRPG_Inventory _array_element)) (.ItemID (Utilities|Struct|BreakSRPG_IDItem _returnvalue)))
              _)))))))

(event Custom|Save%20Inventories
  (params (Inventories :type Array%20of%20Actor%20Object%20References))
  (for _array_element Inventories
    (bind (_itemid _name _description _bstack _keywords _buycost _sellcost _stack _maxstack _types) (Class|BPIRPGBaseInfo|GetBaseInfo(Message) _array_element))
    (Variables|Default|SetSItemType "NewEnumerator0")
    (for _array_element_2 _types
      (Utilities|FlowControl|Sequence
        (:then_0
          (if (Utilities|Enum|Equal(Enum) _array_element_2 "equip")
            (Variables|Default|SetSItemType "NewEnumerator1")))
        (:then_1
          (if (Utilities|Enum|Equal(Enum) _array_element_2 "weapon")
            (Variables|Default|SetSItemType "NewEnumerator1")))))
    (Utilities|Array|Add (Variables|Default|GetSPlayer%20Inventories) (Utilities|Struct|MakeSRPG_Inventory _itemid 0 _name _description (Variables|Default|GetSItemType) _stack))
    (Development|PrintString 0 (Utilities|String|Append "ID:" _itemid "=" "Name:" _name) true true "(R=1.000000,G=0.674767,B=0.000000,A=1.000000)")))

(fn GetPlayerInventories
  (return 0))

(fn SetPlayerInventories
  (params (In%20Inventories :type Array%20of%20Actor%20Object%20References)))

(fn GetOpenLevel
  (return (Variables|Default|GetOpen%20Level%20Name)))

(fn SetOpenLevel
  (params (In%20Name :type String))
  (Variables|Default|SetOpen%20Level%20Name In%20Name))

(fn GetPlayerName
  (return (Variables|Default|GetPlayerName)))

(fn SetPlayerName
  (params (In%20Name :type String))
  (Variables|Default|SetPlayerName In%20Name))

(fn GetStructPlayerInventories
  (return (Variables|Default|GetSPlayer%20Inventories)))