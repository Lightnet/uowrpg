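; BPRPG_PlayerSaveGameInfo is a save-game data object that holds one RPG player's persistent state.
; SavePlayerState copies name, status, stats, skills, quests, hotkeys, support requests, storage and inventories from the player state, optionally storing the player's transform.
; Accessors expose the open level name, player name and inventory struct, while GetPlayerInventories and SetPlayerInventories are empty stubs.
; The asset only captures data, with no disk writing or restore logic.
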(event Custom|Save%20PlayerState
  (params (playerstate :type BPRPG%20Player%20State%20Object%20Reference) (Player%20Transform :type Transform) (IsSavePosition :type Boolean))
  ;[1 1 1] Save Stucts
  (if IsSavePosition
    (Variables|LevelMap|SetPlayer%20Transform Player%20Transform))
  (Variables|PlayerStatus|SetPlayerName (Variables|/Game/Uorpg/Blueprints/Game/GameModeRPG/BPRPG_PlayerState.BPRPG_PlayerState_C|GetPlayer playerstate))
  (Variables|PlayerStatus|SetPlayer%20Status (Variables|/Game/Uorpg/Blueprints/Game/GameModeRPG/BPRPG_PlayerState.BPRPG_PlayerState_C|GetPlayerStatus playerstate))
  (Variables|PlayerStatus|SetPlayer%20Stats (Variables|/Game/Uorpg/Blueprints/Game/GameModeRPG/BPRPG_PlayerState.BPRPG_PlayerState_C|GetPlayerStats playerstate))
  (Variables|PlayerItems|SetSSkills (Variables|/Game/Uorpg/Blueprints/Game/GameModeRPG/BPRPG_PlayerState.BPRPG_PlayerState_C|GetSSkills playerstate))
  (Variables|PlayerItems|SetSQuests (Variables|/Game/Uorpg/Blueprints/Game/GameModeRPG/BPRPG_PlayerState.BPRPG_PlayerState_C|GetSQuests playerstate))
  (Variables|PlayerItems|SetSHotkeys (Variables|/Game/Uorpg/Blueprints/Game/GameModeRPG/BPRPG_PlayerState.BPRPG_PlayerState_C|GetSHotkeys playerstate))
  (Variables|PlayerItems|SetSRequestSupports (Variables|/Game/Uorpg/Blueprints/Game/GameModeRPG/BPRPG_PlayerState.BPRPG_PlayerState_C|GetRequestSupport playerstate))
  (Variables|PlayerItems|SetSStorage (Variables|/Game/Uorpg/Blueprints/Game/GameModeRPG/BPRPG_PlayerState.BPRPG_PlayerState_C|GetSStorage playerstate))
  (Variables|PlayerItems|SetSPlayer%20Inventories (Variables|/Game/Uorpg/Blueprints/Game/GameModeRPG/BPRPG_PlayerState.BPRPG_PlayerState_C|GetSPlayer%20Inventories playerstate)))

(fn GetPlayerInventories
  (return 0))

(fn SetPlayerInventories
  (params (In%20Inventories :type Array%20of%20Actor%20Object%20References)))

(fn GetOpenLevel
  (return (Variables|LevelMap|GetOpen%20Level%20Name)))

(fn SetOpenLevel
  (params (In%20Name :type String))
  (Variables|LevelMap|SetOpen%20Level%20Name In%20Name))

(fn GetPlayerName
  (return (Variables|PlayerStatus|GetPlayerName)))

(fn SetPlayerName
  (params (In%20Name :type String))
  (Variables|PlayerStatus|SetPlayerName In%20Name))

(fn GetStructPlayerInventories
  (return (Variables|PlayerItems|GetSPlayer%20Inventories)))